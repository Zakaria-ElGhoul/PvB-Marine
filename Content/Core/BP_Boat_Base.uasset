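; Base boat actor that moves in fixed steps from keyboard input, limited by a Moves counter shown on a TextRender.
; A pressed key is looked up in the DirectionKeys map for a step offset, which a Timeline lerps the location across without sweep.
; Each finished step decrements Moves and chains another while a key remains held.
; Pressing X resets Moves to five.
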(event `self.ReceiveBeginPlay`
  (`TextRenderComponent.K2_SetText` (`self.TextRender`) (`KismetTextLibrary.Conv_IntToText` (stale `Key|X` _output_get)) :!label _label))

(event `Key|X`
  (params (Key :type "Key Structure"))
  (:`Pressed`
    (bind _output_get (set `self.Moves` 5))
    (goto _label)))

(event `TakeNextStep`
  (bind _returnvalue (> (`self.Moves`) 0))
  (bind _output_get (set `self.Start Location` (`self.K2_GetActorLocation`) :!label _label_2))
  (set `self.End Location` (+ _output_get (stale `Key|AnyKey` _output_get)))
  (bind (_direction _alpha) (`Timeline|Timeline` :!via `PlayFromStart`)
    (:`Update`
      (`self.K2_SetActorLocation` (`KismetMathLibrary.VLerp` (`self.Start Location`) (`self.End Location`) _alpha)))
    (:`Finished`
      (if _returnvalue
        (bind _result (`/Engine/EditorBlueprintResources/StandardMacros.DecrementInt` (`self.Moves`))
          (:`  `
            (`TextRenderComponent.K2_SetText` (`self.TextRender`) (`KismetTextLibrary.Conv_IntToText` _result))
            (if (`self.bShouldTakeA Step`)
              (`self.TakeNextStep`))))
        (else
          (set `self.bShouldTakeA Step` _returnvalue))))))

(event `Key|AnyKey`
  (params (Key :type "Key Structure"))
  (bind (_value _returnvalue) (`BlueprintMapLibrary.Map_Find` (`self.DirectionKeys`) Key))
  (:`Pressed`
    (set `self.bShouldTakeA Step` true)
    (if (and _returnvalue (not (`TimelineComponent.IsPlaying` (`self.Timeline`))) (`self.bShouldTakeA Step`) (> (`self.Moves`) 0))
      (bind _output_get (set `self.Direction Step Size` _value))
      (goto _label_2)))
  (:`Released`
    (set `self.bShouldTakeA Step` false)))

(fn `UserConstructionScript`)