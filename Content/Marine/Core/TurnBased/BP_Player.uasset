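; BP_Player is a turn-based player Blueprint that sets up on-screen UI and provides a test input for switching turns.
; On BeginPlay it adds two widgets to the viewport, storing the WBP_PlayerWidget instance as TurnUI.
; Pressing 1 calls SwitchTurn on BP_Gamemode_Turnbased, then has TurnUI update its text.
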(event `self.ReceiveBeginPlay`
  (bind _returnvalue (`|CreateWidget` null))
  (bind _returnvalue_2 (`|CreateWidget` "/Game/Marine/Core/TurnBased/WBP_PlayerWidget.WBP_PlayerWidget_C"))
  (bind _output_get (set `self.TurnUI` _returnvalue_2))
  (`UserWidget.AddToViewport` _output_get 0)
  (`UserWidget.AddToViewport` _returnvalue 0))

(event `Key|One`
  (params (Key :type "Key Structure"))
  ;[1 1 1] Test if switching works
  (:`Pressed`
    (bind _asbp_gamemode_turnbased (cast `/Game/Marine/Core/BP_Gamemode_Turnbased` (`GameplayStatics.GetGameMode`)))
    (`/Game/Marine/Core/BP_Gamemode_Turnbased.SwitchTurn` _asbp_gamemode_turnbased)
    (`/Game/Marine/Core/TurnBased/WBP_PlayerWidget.UpdateText` (`self.TurnUI`))))

(fn `UserConstructionScript`)