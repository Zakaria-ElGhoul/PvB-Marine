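; BP_EnemySpawner populates the turn-based marine game with enemy ships when play begins.
; On BeginPlay it spawns a BP_EnemyShips at every BP_Spawn_Point, adjusting for collisions but always spawning.
; It also binds SpawnEnemy to the BP_Gamemode_Turnbased respawn event.
; SpawnEnemy currently spawns nothing: its loop body is empty, and it only grows the EnemiesSpawned count by an increasing increment.
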(event `self.ReceiveBeginPlay`
  (bind _asbp_gamemode_turnbased (cast `/Game/Marine/Core/TurnBased/BP_Gamemode_Turnbased` (`GameplayStatics.GetGameMode`)))
  (add `/Game/Marine/Core/TurnBased/BP_Gamemode_Turnbased.Respawn Enemies` _asbp_gamemode_turnbased (delegate `SpawnEnemy`))
  (bind _outactors (`GameplayStatics.GetAllActorsOfClass` "/Game/Marine/Core/TurnBased/BP_Spawn_Point.BP_Spawn_Point_C"))
  (for _array_element _outactors
    (`|SpawnActorFromClass` "/Game/Marine/Core/TurnBased/BP_EnemyShips.BP_EnemyShips_C" (`self.GetTransform` _array_element) "AdjustIfPossibleButAlwaysSpawn" "OverrideRootScale" null null)))

(event `SpawnEnemy`
  (for _ (range (`self.EnemiesSpawned`))
    _)
  (`/Engine/EditorBlueprintResources/StandardMacros.IncrementInt` (`self.IncrementEnemies`)
    (:`  `
      (set `self.EnemiesSpawned` (+ (`self.EnemiesSpawned`) (`self.IncrementEnemies`))))))

(fn `UserConstructionScript`)