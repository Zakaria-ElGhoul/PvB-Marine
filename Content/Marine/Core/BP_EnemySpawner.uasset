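; BP_EnemySpawner is a spawner actor that creates waves of enemy AI boats at its own transform.
; On BeginPlay it binds SpawnEnemy to the respawn event of BP_WaveSystemGameMode.
; Each call spawns the current count of BP_EnemyBoatAI, adjusting for collisions but always spawning.
; It then raises the increment by one and adds it to the count, so successive waves grow at an accelerating rate.
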(event `self.ReceiveBeginPlay`
  (bind _asbp_wave_system_game_mode (cast `/Game/Marine/Blueprints/EnemyWaveSystem/BP_WaveSystemGameMode` (`GameplayStatics.GetGameMode`)))
  (add `/Game/Marine/Blueprints/EnemyWaveSystem/BP_WaveSystemGameMode.RespawnEnemies` _asbp_wave_system_game_mode (delegate `SpawnEnemy`)))

(event `SpawnEnemy`
  (for _ (range (`self.EnemiesSpawned`))
    (`|SpawnActorFromClass` "/Game/Marine/Blueprints/EnemyWaveSystem/BP_EnemyBoatAI.BP_EnemyBoatAI_C" (`self.GetTransform`) "AdjustIfPossibleButAlwaysSpawn" "OverrideRootScale" null null))
  (`/Engine/EditorBlueprintResources/StandardMacros.IncrementInt` (`self.IncrementEnemies`)
    (:`  `
      (set `self.EnemiesSpawned` (+ (`self.EnemiesSpawned`) (`self.IncrementEnemies`))))))

(fn `UserConstructionScript`)