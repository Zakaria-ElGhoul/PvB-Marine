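; BP_DamageCalculator works out the damage multiplier for an incoming damage type against a set of target damage types.
; DamageMultiplier uses the incoming enum's name as the row key into DT_DamageTable, then looks up each target type in that row's Type1 map.
; All matched values are multiplied together into one combined multiplier.
; A missing row returns a neutral multiplier, leaving damage unscaled.
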(fn `DamageMultiplier`
  (params (IncomingDamage :type "/Game/Marine/Core/DamageTypes/Enum_AttackTypes Enum" :default "NewEnumerator0") (DamageTypes :type "Array of /Game/Marine/Core/DamageTypes/Enum_AttackTypes Enum"))
  (returns (Current_Multi1 :type "Float (double-precision)"))
  (locals (Damage_Mult :type "Array of Float (double-precision)") (Current_Multi :type "Float (double-precision)" :default 1.0))
  ;[1 1 1] Checks in damage table if attack type is present
  (bind _returnvalue (`|GetDataTableRow` "/Game/Marine/Core/DamageTypes/DT_DamageTable.DT_DamageTable" (`KismetStringLibrary.Conv_StringToName` (`|GetEnumeratorNameAsString` IncomingDamage)))
    (:`then`
      (for _array_element DamageTypes
        (bind (_value _returnvalue_2) (`BlueprintMapLibrary.Map_Find` (`.Type1_5_D69829544E9EDFC5DDD645B572B59849` (break `/Game/Marine/Core/DamageTypes/Struct_DamageType` _returnvalue)) _array_element))
        (if _returnvalue_2
          (`KismetArrayLibrary.Array_Add` (`local.Damage_Mult`) _value)))
      ;[1 1 1] Adds multiplier to damage
      (for _array_element_2 (`local.Damage_Mult`)
        (set `local.Current_Multi` (* _array_element_2 (`local.Current_Multi`))))
      (return (`local.Current_Multi`)))
    (:`RowNotFound`
      (return 1.0) ; If no row has been found, it will return no multiplier
    )))