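; Visual attack projectile for turn-based ship combat, fired by either player or enemy ships.
; OnInitializeProjectile stores endpoints and impact assets, then a timeline drives VInterpTo toward the destination, using a distance check rather than physical collision.
; On arrival it triggers the target ship's game-feel hit reaction and calls OnCollision.
; OnCollision plays screen flash, impact VFX (smoke fallback) and sound, notifies the game mode the attack effect ended, then destroys itself.
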(event `self.ReceiveBeginPlay`
  (`GameplayStatics.PlaySound2D` "/Game/Marine/Audio/AttackSounds/MetaSounds/MS_ShotSound.MS_ShotSound" 1.0 1.0 0.0 null null))

(event `OnInitializeProjectile`
  (params (IsPlayerProjectile :type Boolean) (StartPos :type "Vector Structure") (EndDestination :type "Vector Structure") (Target :type "Object Object Reference") (ImpactVFX :type "NiagaraSystem Object Reference") (ImpactSound :type "MetaSoundSource Object Reference"))
  (set `self.Impact VFX` ImpactVFX)
  (set `self.Impact Sound` ImpactSound)
  (set `self.IsPlayerProj` IsPlayerProjectile)
  (set `self.End Destination` EndDestination)
  (set `self.Start Pos` StartPos)
  (set `self.HasInitialized` true)
  (bind (_direction _newtrack_0) (`Timeline|ProjectileMove` :!via `PlayFromStart` :!label _label)
    (:`Update`
      (if (< (`KismetMathLibrary.Vector_Distance` (`self.K2_GetActorLocation`) (`self.End Destination`)) 5.0)
        (`|ExecutionSequence`
          (:`then_0`
            (goto _label :!via `Stop`))
          (:`then_1`
            (if (`self.IsPlayerProj`)
              (bind _asbp_enemy_ship (cast `/Game/Marine/Core/TurnBasedSystem/BP_EnemyShip` Target)
                (:`then`
                  (`/Game/Marine/Core/AttackVisual/AC_GameFeel.OnHit` (`/Game/Marine/Core/TurnBasedSystem/BP_ShipBase.AC_GameFeel` _asbp_enemy_ship))
                  (`self.OnCollision` (`self.IsPlayerProj`) :!label _label_2))
                (:`CastFailed`
                  (`KismetSystemLibrary.PrintString` "KANKER")))
              (else
                (bind _asbp_allied_ship (cast `/Game/Marine/Core/TurnBasedSystem/BP_AlliedShip` Target))
                (`/Game/Marine/Core/AttackVisual/AC_GameFeel.OnHit` (`/Game/Marine/Core/TurnBasedSystem/BP_ShipBase.AC_GameFeel` _asbp_allied_ship))
                (goto _label_2)))))
        (else
          (`self.K2_SetActorLocation` (`KismetMathLibrary.VInterpTo` (`self.Start Pos`) (`self.End Destination`) _newtrack_0 10.0)))))
    (:`Finished`
      (`self.K2_SetActorLocation` (`self.End Destination`)))))

(fn `OnCollision`
  (params (IsPlayerTurn :type Boolean))
  (bind _impact_vfx (`self.Impact VFX`))
  (bind _returnvalue (`SceneComponent.K2_GetComponentLocation` (`self.Sphere`)))
  (`/Game/Marine/Core/AttackVisual/WBP_WhiteFlashEffect.OnWhiteFlash` (`/Game/Marine/Core/TurnBasedSystem/BP_Gamemode_Turnbased.WhiteFlashEffect` (cast `/Game/Marine/Core/TurnBasedSystem/BP_Gamemode_Turnbased` (`GameplayStatics.GetGameMode`) :!pure true)))
  (`/Engine/EditorBlueprintResources/StandardMacros.IsValid` _impact_vfx
    (:`Is Valid`
      (`NiagaraFunctionLibrary.SpawnSystemAtLocation` _impact_vfx _returnvalue))
    (:`Is Not Valid`
      (`GameplayStatics.SpawnEmitterAtLocation` "/Game/Marine/Effects/AttackEffects/LandSmoke_LParticle.LandSmoke_LParticle" _returnvalue (struct) (5.0 5.0 5.0))))
  (`/Engine/EditorBlueprintResources/StandardMacros.IsValid` (`self.Impact Sound`)
    (:`Is Valid`
      (`GameplayStatics.PlaySound2D` (`self.Impact Sound`) 1.0 1.0 0.0 null null))
    (:`Is Not Valid`
      (`GameplayStatics.PlaySound2D` "/Game/Marine/Audio/AttackSounds/MetaSounds/ImpactSound.ImpactSound" 1.0 1.0 0.0 null null)))
  (message `/Game/Marine/Core/AttackVisual/BPI_AttackEffects.OnEndAttackEffect` (`GameplayStatics.GetGameMode`) IsPlayerTurn)
  (`self.K2_DestroyActor`))

(fn `UserConstructionScript`)