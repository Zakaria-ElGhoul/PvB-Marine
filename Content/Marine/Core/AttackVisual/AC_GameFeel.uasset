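; AC_GameFeel is a component that supplies attack and healing feedback for the turn-based game.
; ShootProjectile spawns a BP_Projectile aimed at its destination and passes it the target and impact effects, while HealUnit spawns a Niagara healing effect.
; OnHit triggers the game mode's white flash and a hit stop through near-zero global time dilation.
; A tiny timer, stretched by that dilation, restores normal time and plays a camera shake.
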(event `self.ReceiveBeginPlay`
  (bind _asbp_gamemode_turnbased (cast `/Game/Marine/Core/TurnBasedSystem/BP_Gamemode_Turnbased` (`GameplayStatics.GetGameMode`)))
  (set `self.As BP Gamemode Turnbased` _asbp_gamemode_turnbased))

(event `ShootProjectile`
  (params (IsPlayerProjectile :type Boolean) (SpawnTransform :type "Transform Structure") (EndDestination :type "Vector Structure") (Target :type "Object Object Reference") (ImpactVFX :type "NiagaraSystem Object Reference") (ImpactSound :type "MetaSoundSource Object Reference"))
  (bind _location (.location SpawnTransform))
  (bind _returnvalue (`|SpawnActorFromClass` "/Game/Marine/Core/AttackVisual/BP_Projectile.BP_Projectile_C" (`KismetMathLibrary.MakeTransform` _location (`KismetMathLibrary.FindLookAtRotation` _location EndDestination) (.scale SpawnTransform)) "Undefined" "OverrideRootScale" null null))
  (`/Game/Marine/Core/AttackVisual/BP_Projectile.OnInitializeProjectile` _returnvalue IsPlayerProjectile (0.0 0.0 0.0) EndDestination Target ImpactVFX ImpactSound))

(event `HealUnit`
  (params (Location :type "Vector Structure"))
  (`NiagaraFunctionLibrary.SpawnSystemAtLocation` "/Game/Marine/Effects/AttackEffects/NiagaraHealing.NiagaraHealing" Location))

(event `OnHit`
  (`/Game/Marine/Core/AttackVisual/WBP_WhiteFlashEffect.OnWhiteFlash` (`/Game/Marine/Core/TurnBasedSystem/BP_Gamemode_Turnbased.WhiteFlashEffect` (`self.As BP Gamemode Turnbased`)))
  (`GameplayStatics.SetGlobalTimeDilation` 0.001)
  (`KismetSystemLibrary.K2_SetTimerDelegate` (delegate `EndHitStop`) 0.0004))

(event `EndHitStop`
  (`GameplayStatics.SetGlobalTimeDilation` 1.0)
  (`GameplayStatics.PlayWorldCameraShake` "/Game/Marine/Core/AttackVisual/CS_ImpactShake.CS_ImpactShake_C" (`PlayerCameraManager.GetCameraLocation` (`GameplayStatics.GetPlayerCameraManager` 0)) 0.0 1800.0))