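; BP_CardHolder spawns and manages the player's cards at "CardSpot" child actor components on the level's Cam actor.
; Each spawned card gets its visuals and stats from a random DT_Cards row, and Space rerolls them all for debugging.
; Tick circle-casts for a card to drive hover start and end on the selected one.
; Left mouse press and release broadcast drag start and end to every card.
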(event `self.ReceiveBeginPlay`
  ;[1 1 1] Places cards and enables input
  (bind _returnvalue (`GameplayStatics.GetActorOfClass` "/Game/Marine/Core/UnitStatSystem/Cam.Cam_C"))
  (`/Engine/EditorBlueprintResources/StandardMacros.IsValid` _returnvalue
    (:`Is Valid`
      (bind _output_get (set `self.Cam` _returnvalue))
      (set `self.CardPoschildren` (`self.GetComponentsByTag` _output_get "/Script/Engine.ChildActorComponent" "CardSpot"))
      (`self.PlaceCard`)
      (`self.EnableInput` (`GameplayStatics.GetPlayerController` 0)))
    (:`Is Not Valid`
      (`KismetSystemLibrary.PrintString` "No Cam actor found! place cam actor from the Unitstat folder!" true true (struct :`R` 1.0 :`B` 0.008127 :`A` 1.0) 50.0))))

(event `self.ReceiveTick`
  (params (DeltaSeconds :type "Float (single-precision)"))
  (bind _selectedcard (`self.SelectedCard`))
  ;[1 1 1] LineTrace to check cards
  (bind _hitactor (`/Game/Developers/Milan/Collections/CAerdSystewm/3D_Cards/BPFL_CardCast.CircleCastCard` 1.0))
  (bind _asbp_card (cast `/Game/Marine/Core/CardSystem/BP_Card` _hitactor)
    (:`then`
      (`/Engine/EditorBlueprintResources/StandardMacros.IsValid` _asbp_card
        (:`Is Valid`
          (if (== _asbp_card (`self.SelectedCard`))
            (bind _output_get (set `self.SelectedCard` _asbp_card :!label _label))
            (`/Game/Marine/Core/CardSystem/BP_Card.CursorOver` _output_get)
            (else
              (`/Engine/EditorBlueprintResources/StandardMacros.IsValid` _asbp_card
                (:`Is Valid`
                  ;;[1 1 1] connections must be in this order
                  (`|ExecutionSequence`
                    (:`then_0`
                      (`/Engine/EditorBlueprintResources/StandardMacros.IsValid` _selectedcard :!label _label_2
                        (:`Is Valid`
                          (`/Game/Marine/Core/CardSystem/BP_Card.EndCursorOver` _selectedcard :!label _label_3))))
                    (:`then_1`
                      (goto _label))))))))
        (:`Is Not Valid`
          (goto _label_2))))
    (:`CastFailed`
      (`/Engine/EditorBlueprintResources/StandardMacros.IsValid` _selectedcard
        (:`Is Valid`
          (goto _label_3))))))

(event `Key|LeftMouseButton`
  (params (Key :type "Key Structure"))
  ;[1 1 1] Drags card when clicked on
  (:`Pressed`
    (for _array_element (`self.Cards`)
      (`/Game/Marine/Core/CardSystem/BP_Card.OnDrag` _array_element)))
  (:`Released`
    (for _array_element_2 (`self.Cards`)
      (`/Game/Marine/Core/CardSystem/BP_Card.OnEndDrag` _array_element_2))))

(event `Key|SpaceBar`
  (params (Key :type "Key Structure"))
  ;[1 1 1] Debug shuffle cards
  (:`Pressed`
    (for _array_element (`self.Cards`)
      (`self.GenerateCard` _array_element))))

(fn `GenerateCard`
  (params (Card :type "/Game/Marine/Core/CardSystem/BP_Card Object Reference"))
  (bind _outrownames (`DataTableFunctionLibrary.GetDataTableRowNames` "/Game/Marine/Core/CardSystem/DT_Cards.DT_Cards"))
  (bind _returnvalue (`|GetDataTableRow` "/Game/Marine/Core/CardSystem/DT_Cards.DT_Cards" (`KismetArrayLibrary.Array_Random` _outrownames))
    (:`then`
      (bind (_name _description _unitimage _cardvisual _cost _effectamountamount _type) (break `/Game/Marine/Core/CardSystem/S_CardValues` _returnvalue))
      (`/Game/Marine/Core/CardSystem/BP_Card.setCardVisuals` Card _name _description _unitimage _cardvisual _cost _effectamountamount _type))))

(fn `PlaceCard`
  (locals (Quantity :type Integer :default 4))
  ;[1 1 1] Goes trough all cardpositions of cam to place the cards on the correct place
  (for _index (range (+ (`local.Quantity`) 1))
    (bind (_returnvalue_location _returnvalue_rotation) (`KismetMathLibrary.BreakTransform` (`SceneComponent.K2_GetComponentToWorld` (`|GetArrayItem` (`self.CardPoschildren`) _index))))
    (bind _returnvalue (`|SpawnActorFromClass` "/Game/Marine/Core/CardSystem/BP_Card.BP_Card_C" (`KismetMathLibrary.MakeTransform` _returnvalue_location (`KismetMathLibrary.MakeRotator` (+ (.roll _returnvalue_rotation) (`self.CardXRotSpawnDegree`)) 0.0 (- (.yaw _returnvalue_rotation) 90.0))) "Undefined" "OverrideRootScale" null null))
    (`KismetArrayLibrary.Array_Add` (`self.Cards`) _returnvalue)
    (`self.GenerateCard` _returnvalue))
  (return))

(fn `UserConstructionScript`)