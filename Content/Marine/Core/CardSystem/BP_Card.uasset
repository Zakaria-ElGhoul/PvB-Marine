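; Playable card actor that the player drags onto a ship to apply its type, effect and cost.
; Hover plays a timeline that eases the mesh up from its start position.
; While dragged, Tick follows the deprojected mouse; release snaps back, circle-casts for a BP_ShipBase, passes values and hides the card.
; SetCardVisuals fills texts and dynamic material textures and re-shows the card, though Cost text displays the effect amount.
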(event `self.ReceiveBeginPlay`
  (bind (_returnvalue_location _returnvalue_rotation) (`KismetMathLibrary.BreakTransform` (`self.GetTransform`)))
  ;[1 1 1] Sets card values
  (set `self.BeginPos` _returnvalue_location)
  (set `self.BeginRot` _returnvalue_rotation)
  (bind _returnvalue (`PrimitiveComponent.CreateDynamicMaterialInstance` (`self.StaticMesh`) 0 "/Game/Marine/MaterialLibrary/Card/Mat_Card.Mat_Card" "None"))
  (set `self.CardMaterial` _returnvalue))

(event `CursorOver`
  ;[1 1 1] Gives card highlight animation when cursor is hovering
  (if (not (`self.IsDragging`))
    (if (not (`self.HighLighted`))
      (set `self.HighLighted` true)
      (bind (_direction _newtrack_0) (`Timeline|BeginHighLight` :!via `PlayFromStart` :!label _label)
        (:`Update`
          (`SceneComponent.K2_SetWorldLocation` (`self.StaticMesh`) (`|EaseFunction` "ExpoOut" (`KismetMathLibrary.FClamp` _newtrack_0 0.0 0.1) (`self.BeginPos`) (`KismetMathLibrary.MakeVector` (- (.x (`self.BeginPos`)) (- 15.0 (`self.MaxForward`))) (.y (`self.BeginPos`)) (+ (.z (`self.BeginPos`)) 13.0))) false false))))))

(event `EndCursorOver`
  ;[1 1 1] Gives card highlight animation when cursor is hovering
  (if (not (`self.IsDragging`))
    (if (`self.HighLighted`)
      (set `self.HighLighted` false)
      (goto _label :!via `ReverseFromEnd`))))

(event `OnDrag`
  ;[1 1 1] set card state to drag card
  (if (`self.HighLighted`)
    (`SceneComponent.K2_SetWorldLocation` (`self.StaticMesh`) (`self.BeginPos`) false false)
    (set `self.IsDragging` true)))

(event `OnEndDrag`
  ;[1 1 1] Resets cards state if no valid target has been found, else it wil send data to target
  (if (`self.IsDragging`)
    (set `self.IsDragging` false)
    (`self.K2_SetActorLocation` (`self.BeginPos`))
    (bind _hitactor (`/Game/Marine/Core/CardSystem/BPFL_CardCast.CircleCastCard` 5.0))
    (bind _asbp_ship_base (cast `/Game/Marine/Core/TurnBasedSystem/BP_ShipBase` _hitactor))
    (`/Game/Marine/Core/TurnBasedSystem/BP_ShipBase.Set Ship Values` _asbp_ship_base (`self.CardType`) (`self.CardEffectAmount`) (`self.CardCost`))
    (`SceneComponent.SetVisibility` (`self.ChildActor`) false true)
    (`PrimitiveComponent.SetCollisionResponseToChannel` (`self.Box`) "ECC_Visibility" "ECR_Ignore")))

(event `self.ReceiveTick`
  (params (DeltaSeconds :type "Float (single-precision)"))
  (bind _returnvalue (`WidgetLayoutLibrary.GetViewportScale`))
  ;[1 1 1] Drags card if 'IsDragging' = true
  (if (`self.IsDragging`)
    (bind _returnvalue_2 (`WidgetLayoutLibrary.GetMousePositionOnViewport`))
    (bind (_worldposition _worlddirection) (`GameplayStatics.DeprojectScreenToWorld` (`GameplayStatics.GetPlayerController` 0) (* _returnvalue_2 (`KismetMathLibrary.MakeVector2D` _returnvalue _returnvalue))))
    (`self.K2_SetActorLocationAndRotation` (- (+ _worldposition (* _worlddirection 10.0)) (0.0 0.0 4.0)) (`self.BeginRot`))))

(fn `setCardVisuals`
  (params (CardName :type String) (CardDescription :type String) (CardUnitImage :type "Texture2D Object Reference") (CardVisual :type "Texture2D Object Reference") (CardCost :type Integer) (CardEffectAmount :type Integer) (CardType :type "/Game/Marine/Core/CardSystem/E_CardType Enum" :default "NewEnumerator0"))
  (set `self.CardName` CardName)
  (set `self.CardDescription` CardDescription)
  (set `self.CardUnitImage` CardUnitImage)
  (set `self.CardVisual` CardVisual)
  (set `self.CardCost` CardCost)
  (set `self.CardEffectAmount` CardEffectAmount)
  (set `self.CardType` CardType)
  (`TextRenderComponent.K2_SetText` (`self.Name`) (`KismetTextLibrary.Conv_StringToText` (`self.CardName`)))
  (`TextRenderComponent.K2_SetText` (`self.Effect`) (`KismetTextLibrary.Conv_IntToText` (`self.CardEffectAmount`)))
  (`TextRenderComponent.K2_SetText` (`self.Cost`) (`KismetTextLibrary.Conv_IntToText` (`self.CardEffectAmount`)))
  (`MaterialInstanceDynamic.SetTextureParameterValue` (`self.CardMaterial`) "Unit" (`self.CardUnitImage`))
  (`MaterialInstanceDynamic.SetTextureParameterValue` (`self.CardMaterial`) "CardVisuals" (`self.CardVisual`))
  (`SceneComponent.SetVisibility` (`self.ChildActor`) true true)
  (`PrimitiveComponent.SetCollisionResponseToChannel` (`self.Box`) "ECC_Visibility" "ECR_Block"))

(fn `UserConstructionScript`)