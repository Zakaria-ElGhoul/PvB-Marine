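; BP_EnemyCardHolder spawns the enemy's hand of cards and deals random card data to it.
; On BeginPlay it finds BP_Cam and spawns BP_EnemyCard actors at its child actor components tagged EnemyCardSpot, adjusting their rotation.
; Each card's visuals and stats are set from a random DT_Cards row.
; AddMissingCards re-rolls existing cards in a specific CardState in place, rather than spawning new actors.
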(event `self.ReceiveBeginPlay`
  ;[1 1 1] Places cards and enables input
  (bind _returnvalue (`GameplayStatics.GetActorOfClass` "/Game/Marine/Core/UnitStatSystem/BP_Cam.BP_Cam_C"))
  (`/Engine/EditorBlueprintResources/StandardMacros.IsValid` _returnvalue
    (:`Is Valid`
      (bind _output_get (set `self.Cam` _returnvalue))
      (set `self.CardPosChildren` (`self.GetComponentsByTag` _output_get "/Script/Engine.ChildActorComponent" "EnemyCardSpot"))
      (`self.PlaceCards`))
    (:`Is Not Valid`
      (`KismetSystemLibrary.PrintString` "No Cam actor found! place cam actor from the Unitstat folder!" true true (struct :`R` 1.0 :`B` 0.008127 :`A` 1.0) 50.0))))

(event `AddMissingCards`
  ;[1 1 1] Hand out new cards
  (for _array_element (`self.Cards`)
    (if (`|EnumEquality` (`/Game/Marine/Core/EnemyCardSystem/BP_EnemyCard.CardState` _array_element) "NewEnumerator1")
      (`self.GenerateCard` _array_element))))

(fn `GenerateCard`
  (params (EnemyCard :type "/Game/Marine/Core/EnemyCardSystem/BP_EnemyCard Object Reference"))
  (bind _outrownames (`DataTableFunctionLibrary.GetDataTableRowNames` "/Game/Marine/Core/CardSystem/DT_Cards.DT_Cards"))
  (bind _returnvalue (`|GetDataTableRow` "/Game/Marine/Core/CardSystem/DT_Cards.DT_Cards" (`KismetArrayLibrary.Array_Random` _outrownames))
    (:`then`
      (bind (_name _description _unitimage _cardvisual _cost _effectamountamount _type) (break `/Game/Marine/Core/CardSystem/S_CardValues` _returnvalue))
      (`/Game/Marine/Core/EnemyCardSystem/BP_EnemyCard.setCardVisuals` EnemyCard _name _description _unitimage _cardvisual _cost _effectamountamount _type "NewEnumerator0"))))

(fn `PlaceCards`
  (locals (Quantity :type Integer :default 3))
  (for _index (range (+ (`local.Quantity`) 1))
    (bind (_returnvalue_location _returnvalue_rotation) (`KismetMathLibrary.BreakTransform` (`SceneComponent.K2_GetComponentToWorld` (`|GetArrayItem` (`self.CardPoschildren`) _index))))
    (bind _returnvalue (`|SpawnActorFromClass` "/Game/Marine/Core/EnemyCardSystem/BP_EnemyCard.BP_EnemyCard_C" (`KismetMathLibrary.MakeTransform` _returnvalue_location (`KismetMathLibrary.MakeRotator` (+ (.roll _returnvalue_rotation) (`self.CardXRot`)) 0.0 (- (.yaw _returnvalue_rotation) 90.0))) "Undefined" "OverrideRootScale" null null))
    (`KismetArrayLibrary.Array_Add` (`self.Cards`) _returnvalue)
    (`self.GenerateCard` _returnvalue))
  (return))

(fn `UserConstructionScript`)