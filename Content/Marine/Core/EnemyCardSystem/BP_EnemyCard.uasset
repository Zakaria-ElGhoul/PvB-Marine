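; BP_EnemyCard is an enemy card actor in the card system, showing a name, numbers and artwork on a mesh.
; BeginPlay stores the starting transform and creates a dynamic material for the card mesh.
; SetCardVisuals stores card data, updates texts and texture parameters, shows the child actor and resets CardState; the Cost text displays the effect amount, not CardCost.
; OnUsed hides the child actor and resets CardState, without any targeting logic.
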(event `self.ReceiveBeginPlay`
  (bind (_returnvalue_location _returnvalue_rotation) (`KismetMathLibrary.BreakTransform` (`self.GetTransform`)))
  ;[1 1 1] Sets card values
  (set `self.BeginPos` _returnvalue_location)
  (set `self.BeginRot` _returnvalue_rotation)
  (bind _returnvalue (`PrimitiveComponent.CreateDynamicMaterialInstance` (`self.StaticMesh`) 0 null "None"))
  (set `self.CardMaterial` _returnvalue))

(event `OnUsed`
  ;[1 1 1] Resets cards state if no valid target has been found, else it wil send data to target
  (`SceneComponent.SetVisibility` (`self.ChildActor`) false true)
  (set `self.CardState` 0))

(fn `setCardVisuals`
  (params (CardName :type String) (CardDescription :type String) (CardUnitImage :type "Texture2D Object Reference") (CardVisual :type "Texture2D Object Reference") (CardCost :type Integer) (CardEffectAmount :type Integer) (CardType :type "/Game/Marine/Core/CardSystem/E_CardType Enum" :default "NewEnumerator0") (AttackType :type "/Game/Marine/Core/DamageTypes/Enum_AttackTypes Enum" :default "NewEnumerator0"))
  (set `self.CardName` CardName)
  (set `self.CardDescription` CardDescription)
  (set `self.CardUnitImage` CardUnitImage)
  (set `self.CardVisual` CardVisual)
  (set `self.CardCost` CardCost)
  (set `self.CardEffectAmount` CardEffectAmount)
  (set `self.CardType` CardType)
  (set `self.AttackType` AttackType)
  (`TextRenderComponent.K2_SetText` (`self.Name`) (`KismetTextLibrary.Conv_StringToText` (`self.CardName`)))
  (`TextRenderComponent.K2_SetText` (`self.Effect`) (`KismetTextLibrary.Conv_IntToText` (`self.CardEffectAmount`)))
  (`TextRenderComponent.K2_SetText` (`self.Cost`) (`KismetTextLibrary.Conv_IntToText` (`self.CardEffectAmount`)))
  (`MaterialInstanceDynamic.SetTextureParameterValue` (`self.CardMaterial`) "Unit" (`self.CardUnitImage`))
  (`MaterialInstanceDynamic.SetTextureParameterValue` (`self.CardMaterial`) "CardVisuals" (`self.CardVisual`))
  (`SceneComponent.SetVisibility` (`self.ChildActor`) true true)
  ;[1 1 1] ResetsCardState
  (set `self.CardState` 0))

(fn `UserConstructionScript`)