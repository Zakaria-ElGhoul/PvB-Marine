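; BP_EnemySpawner spawns BP_ShipBase enemy ships at spawn points and handles turn-based wave respawns.
; BeginPlay binds SpawnEnemy to the BP_Gamemode_Turnbased respawn event, then spawns one ship at each BP_Spawn_Point.
; SpawnEnemy reuses that spawn node EnemiesSpawned times, reading the BeginPlay loop's array element without iterating the points again.
; Each wave then raises the count by a growing increment.
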(event `self.ReceiveBeginPlay`
  (bind _asbp_gamemode_turnbased (cast `/Game/Marine/Core/TurnBasedSystem/BP_Gamemode_Turnbased` (`GameplayStatics.GetGameMode`)))
  (add `/Game/Marine/Core/TurnBasedSystem/BP_Gamemode_Turnbased.Respawn Enemies` _asbp_gamemode_turnbased (delegate `SpawnEnemy`))
  (bind _outactors (`GameplayStatics.GetAllActorsOfClass` "/Game/Marine/Core/TurnBasedSystem/BP_Spawn_Point.BP_Spawn_Point_C"))
  (for _array_element _outactors
    (bind (_returnvalue_location _returnvalue_rotation) (`KismetMathLibrary.BreakTransform` (`self.GetTransform` _array_element)))
    (`|SpawnActorFromClass` "/Game/Marine/Core/TurnBasedSystem/BP_ShipBase.BP_ShipBase_C" (`KismetMathLibrary.MakeTransform` _returnvalue_location _returnvalue_rotation (`self.Spawn Transform Scale`)) "AdjustIfPossibleButAlwaysSpawn" "OverrideRootScale" null null :!label _label)))

(event `SpawnEnemy`
  (for _ (range (`self.EnemiesSpawned`))
    (goto _label))
  (`/Engine/EditorBlueprintResources/StandardMacros.IncrementInt` (`self.IncrementEnemies`)
    (:`  `
      (set `self.EnemiesSpawned` (+ (`self.EnemiesSpawned`) (`self.IncrementEnemies`))))))

(fn `UserConstructionScript`)