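; BP_EnemyBoatAI is an enemy boat in the turn-based wave system that is destroyed on colliding with an allied boat.
; On BeginPlay it increments EnemiesAlive in BP_Gamemode_Turnbased.
; A hit from BP_AlliedBoat decrements that count, calls CheckEnemiesLeft and destroys the boat.
; The graph holds no movement or decision logic, and its DamageMultiplier call is unconnected.
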(event `self.ReceiveBeginPlay`
  (bind _asbp_gamemode_turnbased (cast `/Game/Marine/Core/TurnBasedSystem/BP_Gamemode_Turnbased` (`GameplayStatics.GetGameMode`)))
  (`GameplayStatics.GetActorOfClass` "/Game/Marine/Core/EnemyWaveSystem/BP_AlliedBoat.BP_AlliedBoat_C")
  (`/Engine/EditorBlueprintResources/StandardMacros.IncrementInt` (`/Game/Marine/Core/TurnBasedSystem/BP_Gamemode_Turnbased.Enemies Alive` _asbp_gamemode_turnbased)))

(event `self.ReceiveHit`
  (params (MyComp :type "PrimitiveComponent Object Reference") (Other :type "Actor Object Reference") (OtherComp :type "PrimitiveComponent Object Reference") (bSelfMoved :type Boolean) (HitLocation :type "Vector Structure") (HitNormal :type "Vector Structure") (NormalImpulse :type "Vector Structure") (Hit :type "HitResult Structure (by ref)"))
  (bind _asbp_allied_boat (cast `/Game/Marine/Core/EnemyWaveSystem/BP_AlliedBoat` Other))
  (if (== _asbp_allied_boat Hit_HitActor)
    (bind _asbp_gamemode_turnbased (cast `/Game/Marine/Core/TurnBasedSystem/BP_Gamemode_Turnbased` (`GameplayStatics.GetGameMode`)))
    (`/Engine/EditorBlueprintResources/StandardMacros.DecrementInt` (`/Game/Marine/Core/TurnBasedSystem/BP_Gamemode_Turnbased.Enemies Alive` _asbp_gamemode_turnbased)
      (:`  `
        (`/Game/Marine/Core/TurnBasedSystem/BP_Gamemode_Turnbased.CheckEnemiesLeft` _asbp_gamemode_turnbased)
        (`self.K2_DestroyActor`)))))

(fn `UserConstructionScript`)