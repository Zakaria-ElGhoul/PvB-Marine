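; BP_Clickable is a component in the enemy target system that makes its owning actor clickable and outlines it under the cursor.
; On BeginPlay it binds to the owner's click event and caches its static mesh component.
; A click fires OnClicked only when that mesh is valid.
; Cursor-over events toggle the mesh's custom depth rendering for the outline, though their binding to the owner is not shown here.
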(event `self.ReceiveBeginPlay`
  (bind _returnvalue (`self.GetOwner`))
  (bind _returnvalue_2 (`Actor.GetComponentByClass` _returnvalue "/Script/Engine.StaticMeshComponent"))
  ;[1 1 1] Binds mouse events and sets static mesh for outline effect
  (add `Actor.OnClicked` _returnvalue (delegate `OnMouseInput`))
  (`/Engine/EditorBlueprintResources/StandardMacros.IsValid` _returnvalue_2
    (:`Is Valid`
      (set `self.Static Mesh` _returnvalue_2))))

(event `OnMouseInput`
  (params (TouchedActor :type "Actor Object Reference") (ButtonPressed :type "Key Structure" :default "None"))
  ;[1 1 1] Fires a 'On Clicked' event on mouse input
  (`/Engine/EditorBlueprintResources/StandardMacros.IsValid` (`self.Static Mesh`)
    (:`Is Valid`
      (`self.OnClicked`))))

(event `BeginCursorOver`
  (params (TouchedActor :type "Actor Object Reference"))
  ;[1 1 1] Shows outline on object
  (`PrimitiveComponent.SetRenderCustomDepth` (`self.Static Mesh`) true))

(event `EndCursorOver`
  (params (TouchedActor :type "Actor Object Reference"))
  ;[1 1 1] removes outline on object
  (`PrimitiveComponent.SetRenderCustomDepth` (`self.Static Mesh`) false))