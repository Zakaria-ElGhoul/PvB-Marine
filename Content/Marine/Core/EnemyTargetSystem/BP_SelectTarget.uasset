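; BP_SelectTarget provides a cursor pick that finds the clickable target under the mouse.
; SelectTarget multiplies the viewport mouse position by the viewport scale to undo DPI scaling, then deprojects it through player 0's controller.
; A long Visibility line trace follows that ray, and a valid hit actor yields its BP_Clickable component as the result.
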(fn `SelectTarget`
  (returns (ReturnValue :type "/Game/Marine/Core/EnemyTargetSystem/BP_Clickable Object Reference"))
  (bind _returnvalue (`WidgetLayoutLibrary.GetViewportScale` null))
  ;[1 1 1] Select target with cursor
  (bind _returnvalue_2 (`WidgetLayoutLibrary.GetMousePositionOnViewport` null))
  (bind (_worldposition _worlddirection) (`GameplayStatics.DeprojectScreenToWorld` (`GameplayStatics.GetPlayerController` null) (* _returnvalue_2 (`KismetMathLibrary.MakeVector2D` _returnvalue _returnvalue))))
  (bind _outhit (`KismetSystemLibrary.LineTraceSingle` null _worldposition (+ _worldposition (* _worlddirection 2000000.0)) "TraceTypeQuery1"))
  (bind (_bblockinghit _binitialoverlap _time _distance _location _impactpoint _normal _impactnormal _physmat _hitactor) (`GameplayStatics.BreakHitResult` _outhit))
  (`/Engine/EditorBlueprintResources/StandardMacros.IsValid` _hitactor
    (:`Is Valid`
      (return (`Actor.GetComponentByClass` _hitactor "/Game/Marine/Core/EnemyTargetSystem/BP_Clickable.BP_Clickable_C")))))