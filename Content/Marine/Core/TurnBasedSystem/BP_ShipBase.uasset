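; BP_ShipBase is a ship actor in the turn-based system, carrying card type, cost and effect values plus simple health math.
; On BeginPlay it sets its static mesh's custom depth stencil value to 2.
; SetShipValues assigns the card type and accumulates cost and effect amount.
; HealShip returns health plus healing, while DoDamage returns damage minus current health; neither stores the result.
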(event `self.ReceiveBeginPlay`
  (`PrimitiveComponent.SetCustomDepthStencilValue` (`self.StaticMesh`) 2))

(fn `DoDamage`
  (params (DamageAmount :type Integer) (CurrentHealth :type Integer))
  (returns (NewHealth :type Integer))
  (return (- DamageAmount CurrentHealth)))

(fn `HealShip`
  (params (CurrentHealth :type Integer) (HealAmount :type Integer))
  (returns (NewHealth :type Integer))
  (return (+ HealAmount CurrentHealth)))

(fn `SetShipValues`
  (params (CardEffectAmount :type Integer) (`Card Cost` :type Integer) (CardType :type "/Game/Marine/Core/CardSystem/E_CardType Enum" :default "NewEnumerator0"))
  (set `self.CardType` CardType)
  (set `self.CardCost` (+ `Card Cost` (`self.CardCost`)))
  (set `self.CardEffectAmount` (+ CardEffectAmount (`self.CardEffectAmount`)))
  (return))

(fn `UserConstructionScript`)