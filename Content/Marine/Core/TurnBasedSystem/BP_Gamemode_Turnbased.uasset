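; Game mode for a turn-based naval card battle, handling turns, mana, a countdown and win/lose checks.
; A mouse trace drives ship hover and lets a played card fire at an enemy ship; attacks and heals can end the player's turn.
; SwitchTurn alternates sides, checks surviving ships, and grants mana and a card below the mana cap.
; Hits trigger hit stop through near-zero time dilation, with white flash and camera shake.
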(event `OnHit`
  (`/Game/Marine/Core/AttackVisual/WBP_WhiteFlashEffect.OnWhiteFlash` (`self.WhiteFlashEffect`))
  (`GameplayStatics.SetGlobalTimeDilation` 0.001)
  (`KismetSystemLibrary.K2_SetTimerDelegate` (delegate `EndHitStop`) 0.0004))

(event `EndHitStop`
  (`GameplayStatics.SetGlobalTimeDilation` 1.0)
  (`GameplayStatics.PlayWorldCameraShake` "/Game/Marine/Core/AttackVisual/CS_ImpactShake.CS_ImpactShake_C" (`PlayerCameraManager.GetCameraLocation` (`GameplayStatics.GetPlayerCameraManager` 0)) 0.0 1800.0))

(event `Key|LeftMouseButton`
  (params (Key :type "Key Structure"))
  (bind _lastusedcard (`self.LastUsedCard`))
  (bind _shipref (`/Game/Marine/Core/CardSystem/BP_Card.ShipRef` _lastusedcard))
  (bind _location (.location (`self.GetTransform` _shipref)))
  ;[1 1 1] Select a boat to perform a action
  (:`Pressed`
    (bind (_select_target _alliedship _enemyship) (`self.SelectTarget`))
    (`/Engine/EditorBlueprintResources/StandardMacros.IsValid` _enemyship
      (:`Is Valid`
        ;[1 1 1] Some checks to see if target is valid
        (`/Engine/EditorBlueprintResources/StandardMacros.IsValid` (`self.LastUsedCard`)
          (:`Is Valid`
            (if (`self.CardHasBeenPlayed`)
              (if (`|EnumEquality` (`/Game/Marine/Core/CardSystem/BP_Card.CardType` (`self.LastUsedCard`)) "NewEnumerator0")
                ;[1 1 1] Execute Card functions and set variables when the function has executed
                (`/Engine/EditorBlueprintResources/StandardMacros.IsValid` (`/Game/Marine/Core/CardSystem/BP_Card.ShipRef` (`self.LastUsedCard`))
                  (:`Is Valid`
                    (bind _returnvalue (`self.K2_GetActorLocation` _enemyship))
                    (`/Game/Marine/Core/AttackVisual/AC_GameFeel.ShootProjectile` (`/Game/Marine/Core/TurnBasedSystem/BP_ShipBase.AC_GameFeel` _shipref) true (`KismetMathLibrary.MakeTransform` _location (`KismetMathLibrary.FindLookAtRotation` _location _returnvalue) (.scale (`self.GetTransform` _shipref))) _returnvalue _enemyship null null)
                    (`/Game/Marine/Core/AttackSystem/BPFL_OnAttack.Attack Handler Function` _shipref _enemyship _lastusedcard null true)
                    (set `self.CardHasBeenPlayed` false)
                    (`/Game/Marine/Core/TurnBasedSystem/BPFL_TurnStateFunctions.OnEndPlayerTurn` self)))))))))))

(event `HealUnit`
  (bind _lastusedcard (`self.LastUsedCard`))
  (bind _lastusedcard_2 (`self.LastUsedCard`))
  (bind _shipref (`/Game/Marine/Core/CardSystem/BP_Card.ShipRef` _lastusedcard))
  (`/Engine/EditorBlueprintResources/StandardMacros.IsValid` (`self.LastUsedCard`)
    (:`Is Valid`
      (if (`|EnumInequality` (`/Game/Marine/Core/CardSystem/BP_Card.CardState` _lastusedcard) "NewEnumerator1")
        ;[1 1 1] Execute Card functions and set variables when the function has executed
        (`/Engine/EditorBlueprintResources/StandardMacros.IsValid` (`/Game/Marine/Core/CardSystem/BP_Card.ShipRef` _lastusedcard_2)
          (:`Is Valid`
            (`/Game/Marine/Core/AttackSystem/BPFL_OnAttack.Heal Handler Function` (`/Game/Marine/Core/CardSystem/BP_Card.ShipRef` (`self.LastUsedCard`)) (stale `Key|LeftMouseButton` _enemyship) _lastusedcard_2 null true)
            (set `self.CardHasBeenPlayed` false)
            (`/Game/Marine/Core/AttackVisual/AC_GameFeel.HealUnit` (`/Game/Marine/Core/TurnBasedSystem/BP_ShipBase.AC_GameFeel` _shipref) (`self.K2_GetActorLocation` _shipref))
            (`/Game/Marine/Core/TurnBasedSystem/BPFL_TurnStateFunctions.OnEndPlayerTurn` self)))))))

(event `self.ReceiveTick`
  (params (DeltaSeconds :type "Float (single-precision)"))
  (`|ExecutionSequence`
    (:`then_0`
      ;[1 1 1] Timer
      (`KismetSystemLibrary.Delay` 1.0)
      (if (== (`self.Seconds`) 0)
        (if (== (`self.Minutes`) 0)
          (bind _returnvalue (`|CreateWidget` "/Game/Marine/Blueprints/Widgets/WBP_GameOver.WBP_GameOver_C"))
          (`UserWidget.AddToViewport` _returnvalue 0)
          (`GameplayStatics.SetGamePaused` true)
          (else
            (set `self.Seconds` 59)
            (set `self.Minutes` (- (`self.Minutes`) 1))))
        (else
          (set `self.Seconds` (- (`self.Seconds`) 1)))))
    (:`then_1`
      (bind _select_target (`self.SelectTarget`))
      (`/Engine/EditorBlueprintResources/StandardMacros.IsValid` _select_target
        (:`Is Valid`
          (if (== _select_target (`self.Selected Target`))
            (bind _output_get (set `self.Selected Target` _select_target :!label _label))
            (`/Game/Marine/Core/EnemyTargetSystem/BP_Clickable.BeginCursorOver` _output_get null)
            (else
              (`/Engine/EditorBlueprintResources/StandardMacros.IsValid` _select_target
                (:`Is Valid`
                  ;[1 1 1] connections must be in this order
                  (`|ExecutionSequence`
                    (:`then_0`
                      (`/Engine/EditorBlueprintResources/StandardMacros.IsValid` (`self.Selected Target`) :!label _label_2
                        (:`Is Valid`
                          (`/Game/Marine/Core/EnemyTargetSystem/BP_Clickable.EndCursorOver` (`self.Selected Target`) null))))
                    (:`then_1`
                      (goto _label))))))))
        (:`Is Not Valid`
          (goto _label_2))))))

(event `self.ReceiveBeginPlay`
  (`self.EnableInput` (`GameplayStatics.GetPlayerController` 0))
  (bind _returnvalue (`|CreateWidget` "/Game/Marine/Core/AttackVisual/WBP_WhiteFlashEffect.WBP_WhiteFlashEffect_C"))
  (bind _output_get (set `self.WhiteFlashEffect` _returnvalue))
  (`UserWidget.AddToViewport` _output_get 0)
  (bind _returnvalue_2 (`GameplayStatics.GetActorOfClass` "/Game/Marine/Core/CardSystem/BP_CardHolder.BP_CardHolder_C"))
  (set `self.CardHolder` _returnvalue_2))

(event `EnableButton`
  (params (PlayerWBP :type "/Game/Marine/Blueprints/Widgets/WBP_PlayerWidget Object Reference"))
  (`/Engine/EditorBlueprintResources/StandardMacros.IsValid` PlayerWBP
    (:`Is Valid`
      (set `self.PlayerWBP` PlayerWBP))))

(event `CheckEnemiesLeft`
  (bind _outactors (`GameplayStatics.GetAllActorsOfClass` "/Game/Marine/Core/TurnBasedSystem/BP_EnemyShip.BP_EnemyShip_C"))
  (if (== (`KismetArrayLibrary.Array_Length` _outactors) 0)
    (`|CreateWidget` "/Game/Marine/Blueprints/Widgets/WBP_WinGame.WBP_WinGame_C")
    (`GameplayStatics.SetGamePaused` true)))

(event `CheckAlliesLeft`
  (bind _outactors (`GameplayStatics.GetAllActorsOfClass` "/Game/Marine/Core/TurnBasedSystem/BP_AlliedShip.BP_AlliedShip_C"))
  (if (== (`KismetArrayLibrary.Array_Length` _outactors) 0)
    (`|CreateWidget` "/Game/Marine/Blueprints/Widgets/WBP_GameOver.WBP_GameOver_C")
    (`GameplayStatics.SetGamePaused` true)))

(event `/Game/Marine/Core/AttackVisual/BPI_AttackEffects.OnEndAttackEffect`
  (params (IsPlayerTurn :type Boolean))
  (if IsPlayerTurn
    (`/Game/Marine/Core/TurnBasedSystem/BPFL_TurnStateFunctions.OnEndPlayerTurn` self)
    (else
      (`/Game/Marine/Core/TurnBasedSystem/BPFL_TurnStateFunctions.OnEndEnemyTurn` self))))

(fn `CheckHealth`
  (params (CurrentHealth :type Integer) (MaxHealth :type Integer))
  (returns (CanHeal :type Boolean))
  (return (< CurrentHealth MaxHealth)))

(fn `CheckManaCost`
  (params (CurrentMana :type Integer) (CardCost :type Integer))
  (returns (HasEnoughMana :type Boolean))
  (return (>= CurrentMana CardCost)))

(fn `SelectTarget`
  (returns (`Select Target` :type "/Game/Marine/Core/EnemyTargetSystem/BP_Clickable Object Reference") (AlliedShip :type "/Game/Marine/Core/TurnBasedSystem/BP_AlliedShip Object Reference") (EnemyShip :type "/Game/Marine/Core/TurnBasedSystem/BP_EnemyShip Object Reference"))
  (bind _returnvalue (`WidgetLayoutLibrary.GetViewportScale`))
  ;[1 1 1] Select target with cursor
  (bind _returnvalue_2 (`WidgetLayoutLibrary.GetMousePositionOnViewport`))
  (bind (_worldposition _worlddirection) (`GameplayStatics.DeprojectScreenToWorld` (`GameplayStatics.GetPlayerController` 0) (* _returnvalue_2 (`KismetMathLibrary.MakeVector2D` _returnvalue _returnvalue))))
  (bind _outhit (`KismetSystemLibrary.LineTraceSingle` _worldposition (+ _worldposition (* _worlddirection 2000000.0)) "TraceTypeQuery1"))
  (bind (_bblockinghit _binitialoverlap _time _distance _location _impactpoint _normal _impactnormal _physmat _hitactor) (`GameplayStatics.BreakHitResult` _outhit))
  (`/Engine/EditorBlueprintResources/StandardMacros.IsValid` _hitactor
    (:`Is Valid`
      (`|ExecutionSequence`
        (:`then_0`
          (bind _asbp_allied_ship (cast `/Game/Marine/Core/TurnBasedSystem/BP_AlliedShip` _hitactor)))
        (:`then_1`
          (bind _asbp_enemy_ship (cast `/Game/Marine/Core/TurnBasedSystem/BP_EnemyShip` _hitactor))))
      (return (`self.GetComponentByClass` _hitactor "/Game/Marine/Core/EnemyTargetSystem/BP_Clickable.BP_Clickable_C") _asbp_allied_ship _asbp_enemy_ship))))

(fn `SwitchTurn`
  (bind _playerwbp (`self.PlayerWBP`))
  (if (`|EnumEquality` (`self.Current Turn`) "NewEnumerator0")
    (set `self.Current Turn` "NewEnumerator4")
    (`self.CheckAlliesLeft`)
    (`/Game/Marine/Blueprints/Widgets/WBP_PlayerWidget.UpdateText` _playerwbp :!label _label)
    (else
      (set `self.Current Turn` "NewEnumerator0")
      (if (not (== (`self.MaxMana`) (`self.PlayerMana`)))
        (bind _output_get (set `self.PlayerMana` (+ 5 (`self.PlayerMana`))))
        (set `self.CurrentPlayerMana` _output_get)
        (bind _output_get_2 (set `self.EnemyMana` (+ 5 (`self.EnemyMana`))))
        (set `self.CurrentEnemyMana` _output_get_2)
        (`/Game/Marine/Core/CardSystem/BP_CardHolder.GiveCard` (`self.CardHolder`))
        (`Widget.SetIsEnabled` (`/Game/Marine/Blueprints/Widgets/WBP_PlayerWidget.WBP_UI_Button` _playerwbp) true)
        (`self.CheckEnemiesLeft`)
        (goto _label)))))

(fn `UserConstructionScript`)