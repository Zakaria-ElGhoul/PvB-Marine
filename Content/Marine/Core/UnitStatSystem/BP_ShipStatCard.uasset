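; BP_ShipStatCard is an actor that displays an ally or enemy ship's name and HP as a stat card.
; OnCreateCard finds the ship's BP_ShipStatComponent, fills the texts from it and passes itself to OnInitializeStats.
; OnUpdateHP refreshes the HP text, showing zero on death.
; BeginPlay creates a dynamic material for the unit image, but the code that sets its texture and attack text is disconnected.
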(event `self.ReceiveBeginPlay`
  ;[1 1 1] Sets mat instance of stat image
  (bind _returnvalue (`PrimitiveComponent.CreateDynamicMaterialInstance` (`self.UnitImage`) 0 "/Game/Marine/Core/UnitStatSystem/M_StatShipImage.M_StatShipImage" "None"))
  (set `self.MatImage` _returnvalue)
  (set `self.As WBP Ship Stat` null))

(event `OnCreateCard`
  (params (TargetShipAlly :type "/Game/Marine/Core/TurnBasedSystem/BP_AlliedShip Object Reference") (TargetShipEnemy :type "/Game/Marine/Core/TurnBasedSystem/BP_EnemyShip Object Reference") (ShipStatHolder :type "/Game/Marine/Core/UnitStatSystem/BP_ShipStatHolder Object Reference"))
  (bind _shipstatcomponentref (`self.ShipStatcomponentRef`))
  (bind _maxhp (`/Game/Marine/Core/UnitStatSystem/BP_ShipStatComponent.MaxHP` _shipstatcomponentref))
  ;[1 1 1] SetsSta values from stat component
  (`/Engine/EditorBlueprintResources/StandardMacros.IsValid` TargetShipAlly
    (:`Is Valid`
      (bind _output_get (set `self.TargetShip` TargetShipAlly))
      (set `self.ShipStatcomponentRef` (`self.GetComponentByClass` _output_get "/Game/Marine/Core/UnitStatSystem/BP_ShipStatComponent.BP_ShipStatComponent_C")))
    (:`Is Not Valid`
      (bind _output_get_2 (set `self.Target Ship Enemy` TargetShipEnemy))
      (set `self.ShipStatcomponentRef` (`self.GetComponentByClass` _output_get_2 "/Game/Marine/Core/UnitStatSystem/BP_ShipStatComponent.BP_ShipStatComponent_C"))))
  (`/Engine/EditorBlueprintResources/StandardMacros.IsValid` _shipstatcomponentref
    (:`Is Valid`
      (bind _output_get_3 (set `self.CurrentHP` _maxhp))
      (`TextBlock.SetText` (`self.HPText`) (`|FormatText` "HP: {CurrentHP}/{MaxHP}" _output_get_3 _maxhp))
      (`TextBlock.SetText` (`self.ShipNameText`) (`KismetTextLibrary.Conv_StringToText` (`/Game/Marine/Core/UnitStatSystem/BP_ShipStatComponent.ShipName` _shipstatcomponentref)))
      (`/Game/Marine/Core/UnitStatSystem/BP_ShipStatComponent.OnInitializeStats` _shipstatcomponentref self))
    (:`Is Not Valid`
      (`KismetSystemLibrary.PrintString` "ERROR! no BP_shipstat found!"))))

(event `OnUpdateHP`
  (params (CurrentHP :type Integer) (MaxHP :type Integer))
  (if (> CurrentHP 0)
    ;[1 1 1] OnUpdateHP
    (`TextRenderComponent.K2_SetText` (`self.HpText`) (`|FormatText` "HP: {CurrentHP}/{MaxHP}" CurrentHP MaxHP))
    (else
      ;[1 1 1] OnDeath HP
      (`TextRenderComponent.K2_SetText` (`self.HpText`) (`|FormatText` "HP: 0/{MaxHP}" MaxHP)))))

(fn `UserConstructionScript`)