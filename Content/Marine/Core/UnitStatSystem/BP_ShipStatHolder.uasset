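; BP_ShipStatHolder spawns a stat card for every enemy and allied ship in the level.
; A tick after BeginPlay it finds BP_Cam and gathers its child actor components tagged AllySpot and EnemySpot.
; Each BP_ShipStatCard spawns at the spot matching its ship's array index, takes the camera's rotation at a small uniform scale, and receives that ship through OnCreateCard.
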(event `self.ReceiveBeginPlay`
  ;[1 1 1] Gets all statCards of cam
  (`KismetSystemLibrary.DelayUntilNextTick`)
  (bind _returnvalue (`GameplayStatics.GetActorOfClass` "/Game/Marine/Core/UnitStatSystem/BP_Cam.BP_Cam_C"))
  (bind _output_get (set `self.Cam` _returnvalue))
  (set `self.AllySpots` (`self.GetComponentsByTag` _output_get "/Script/Engine.ChildActorComponent" "AllySpot"))
  (set `self.EnemySpots` (`self.GetComponentsByTag` _output_get "/Script/Engine.ChildActorComponent" "EnemySpot"))
  (`self.getAllShips`))

(event `GetAllShips`
  ;[1 1 1] Finds all ships and orders them based on tag
  (bind _outactors (`GameplayStatics.GetAllActorsOfClass` "/Game/Marine/Core/TurnBasedSystem/BP_EnemyShip.BP_EnemyShip_C"))
  (for _array_element _outactors
    (`KismetArrayLibrary.Array_Add` (`self.EnemyUnits`) _array_element))
  (bind _outactors_2 (`GameplayStatics.GetAllActorsOfClass` "/Game/Marine/Core/TurnBasedSystem/BP_AlliedShip.BP_AlliedShip_C"))
  (for _array_element_2 _outactors_2
    (`KismetArrayLibrary.Array_Add` (`self.AllyUnits`) _array_element_2))
  (`|ExecutionSequence`
    (:`then_0`
      ;[1 1 1] Places Enemy unit stats
      (for (_array_element_3 _array_index) (`self.EnemyUnits`)
        (bind (_cardpos _cardrot _cardscale) (`self.StatPlacement` 100.0 _array_index (`|GetArrayItem` (`self.EnemySpots`) _array_index)))
        (bind _returnvalue (`|SpawnActorFromClass` "/Game/Marine/Core/UnitStatSystem/BP_ShipStatCard.BP_ShipStatCard_C" (`KismetMathLibrary.MakeTransform` _cardpos _cardrot _cardscale) "Undefined" "OverrideRootScale" null null))
        (`/Game/Marine/Core/UnitStatSystem/BP_ShipStatCard.OnCreateCard` _returnvalue null _array_element_3)))
    (:`then_1`
      ;[1 1 1] Places Ally unit stats
      (for (_array_element_4 _array_index_2) (`self.AllyUnits`)
        (bind (_cardpos_2 _cardrot_2 _cardscale_2) (`self.StatPlacement` -100.0 _array_index_2 (`|GetArrayItem` (`self.AllySpots`) _array_index_2)))
        (bind _returnvalue_2 (`|SpawnActorFromClass` "/Game/Marine/Core/UnitStatSystem/BP_ShipStatCard.BP_ShipStatCard_C" (`KismetMathLibrary.MakeTransform` _cardpos_2 _cardrot_2 _cardscale_2) "Undefined" "OverrideRootScale" null null))
        (`/Game/Marine/Core/UnitStatSystem/BP_ShipStatCard.OnCreateCard` _returnvalue_2 _array_element_4 null)))))

(fn `StatPlacement`
  (params (CardSideTrans :type "Float (double-precision)") (Index1 :type Integer) (ChildActor :type "ChildActorComponent Object Reference"))
  (returns (CardPos :type "Vector Structure") (CardRot :type "Rotator Structure") (CardScale :type "Vector Structure"))
  (locals (Index :type Integer))
  (set `local.Index` Index1)
  (return (`SceneComponent.K2_GetComponentLocation` ChildActor) (`SceneComponent.K2_GetComponentRotation` (`/Game/Marine/Core/UnitStatSystem/BP_Cam.Camera` (`self.Cam`))) (`KismetMathLibrary.Conv_DoubleToVector` 0.2)))

(fn `UserConstructionScript`)