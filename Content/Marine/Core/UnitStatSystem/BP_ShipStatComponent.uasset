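; Ship stat component that tracks hit points, damage, healing and death for its owning ship.
; HP starts at max, healing is capped there, and each change is pushed to an assigned stat card.
; Damage is scaled by a ship-type multiplier, but new HP is computed as damage minus current HP, reversing the usual subtraction.
; At zero or below, it flags death and calls Die on the BP_ShipBase owner.
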(event `self.ReceiveBeginPlay`
  (set `self.CurrentHP` (`self.MaxHP`)))

(event `OnInitializeStats`
  (params (BP_ShipStatsCard :type "/Game/Marine/Core/UnitStatSystem/BP_ShipStatCard Object Reference"))
  ;[1 1 1] Assign stat card to component
  (set `self.BP_ShipStats` BP_ShipStatsCard))

(event `OnDamage`
  (params (IncomingDamageType :type "/Game/Marine/Core/DamageTypes/Enum_AttackTypes Enum" :default "NewEnumerator0") (IncomingDanageNum :type Integer))
  ;[1 1 1] Sets damage for ship, raises 'isDeath' when HP is below 0
  (bind _current_multi1 (`/Game/Marine/Core/DamageTypes/BP_DamageCalculator.DamageMultiplier` IncomingDamageType (`self.ShipTypes`)))
  (bind _output_get (set `self.CurrentHP` (`KismetMathLibrary.Round` (- (* IncomingDanageNum _current_multi1) (`self.CurrentHP`)))))
  (`/Game/Marine/Core/UnitStatSystem/BP_ShipStatCard.OnUpdateHP` (`self.BP_ShipStats`) _output_get (`self.MaxHP`))
  (if (<= _output_get 0)
    (set `self.IsDeath` true)
    (bind _asbp_ship_base (cast `/Game/Marine/Core/TurnBasedSystem/BP_ShipBase` (`self.GetOwner`))
      (:`then`
        (`/Game/Marine/Core/TurnBasedSystem/BP_ShipBase.Die` _asbp_ship_base))
      (:`CastFailed`
        (`KismetSystemLibrary.PrintString` "Die cast failed in shipstat component" true true (struct :`R` 1.0 :`B` 0.188499 :`A` 1.0) 1000.0)))))

(event `OnHeal`
  (params (IncomingHealNum :type Integer))
  ;[1 1 1] Heals Ship
  (set `self.CurrentHP` (+ IncomingHealNum (`self.CurrentHP`)))
  (if (not (not (> (`self.CurrentHP`) (`self.MaxHP`))))
    (set `self.CurrentHP` (`self.MaxHP`)))
  (`/Game/Marine/Core/UnitStatSystem/BP_ShipStatCard.OnUpdateHP` (`self.BP_ShipStats`) (`self.CurrentHP`) (`self.MaxHP`)))